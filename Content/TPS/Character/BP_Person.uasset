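; BP_Person is a TPS character Blueprint that displays the player's score and network role through widget components.
; On BeginPlay it calls SwitchServer with a hard-coded IP address, then passes itself to the Tag widget's ShowPlayerNetRole.
; Every Tick it casts the ScoreWidget component's user widget and pushes the current Score into it, polling rather than reacting to changes.
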(event EventBeginPlay
  (Class|Person|SwitchServer "192.168.0.174")
  (bind _astag (Utilities|Casting|CastToTag (UserInterface|GetUserWidgetObject (Variables|Default|GetTagWidget))))
  (Class|TagWidget|ShowPlayerNetRole _astag self))

(event Collision|EventActorBeginOverlap
  (params (OtherActor :type Actor%20Object%20Reference)))

(event EventTick
  (params (DeltaSeconds :type Float%20%28single-precision%29))
  (bind _asscore_widget (Utilities|Casting|CastToScoreWidget (UserInterface|GetUserWidgetObject (Variables|Default|GetScoreWidget))))
  (Class|ScoreWidget|ShowScore _asscore_widget (Variables|Default|GetScore)))

(fn ConstructionScript)